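; Mug pickup actor that the player collects with E, recording it as recovered in the PeaceGame game instance.
; A sphere overlap by ThirdPersonCharacterAlternative enables input and shows a PuzzleText prompt, while leaving disables input and removes all widgets.
; Pressing E sets MugRecovered, destroys the actor and plays a sound at its location.
; A MaxItem widget popup sequence is present but never runs.
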(event `self.SphereCollision.OnComponentBeginOverlap`
  (params (OverlappedComponent :type "PrimitiveComponent Object Reference") (OtherActor :type "Actor Object Reference") (OtherComp :type "PrimitiveComponent Object Reference") (OtherBodyIndex :type Integer) (bFromSweep :type Boolean) (SweepResult :type "HitResult Structure (by ref)"))
  ;[1 1 1] Allows the player to interact with object
  (cast `/Game/ThirdPersonBP/Blueprints/ThirdPersonCharacterAlternative` OtherActor)
  (`self.EnableInput` (`GameplayStatics.GetPlayerController` 0))
  (bind _returnvalue (`|CreateWidget` "/Game/Assets/Widgets/PuzzleText.PuzzleText_C"))
  (`UserWidget.AddToViewport` _returnvalue 0))

(event `self.SphereCollision.OnComponentEndOverlap`
  (params (OverlappedComponent :type "PrimitiveComponent Object Reference") (OtherActor :type "Actor Object Reference") (OtherComp :type "PrimitiveComponent Object Reference") (OtherBodyIndex :type Integer))
  ;[1 1 1] Allows the player to interact with object
  (cast `/Game/ThirdPersonBP/Blueprints/ThirdPersonCharacterAlternative` OtherActor)
  (`self.DisableInput` (`GameplayStatics.GetPlayerController` 0))
  (`WidgetLayoutLibrary.RemoveAllWidgets`))

(event `Key|E`
  (params (Key :type "Key Structure"))
  ;[1 1 1] Destroys Actor when E is pressed
  (:`Pressed`
    (bind _aspeace_game (cast `/Game/Assets/Blueprints/GameInstance/PeaceGame` (`GameplayStatics.GetGameInstance`)))
    (set `/Game/Assets/Blueprints/GameInstance/PeaceGame.MugRecovered?` true _aspeace_game)
    (`self.K2_DestroyActor`)
    (`GameplayStatics.PlaySoundAtLocation` "/Game/Assets/Widgets/2022-03-11_08-27-33.2022-03-11_08-27-33" (`self.K2_GetActorLocation`) (struct) 1.0 1.0 0.0 null null null)))

(fn `UserConstructionScript`)