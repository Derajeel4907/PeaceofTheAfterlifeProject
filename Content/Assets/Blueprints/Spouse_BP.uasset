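; Spouse actor that gates the ending: its box trigger checks whether the player has mended at least three memories, tracked in the PeaceGame game instance.
; If so, a timeline scales a particle system, and chained delays off its update reveal the particles and plane, then create an EndCutscene sequence player, with no Play call.
; Otherwise it shows a pictogram, and leaving the box hides pictogram and plane after a delay.
; The quit-after-cutscene nodes are disconnected.
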(event `self.Box.OnComponentBeginOverlap`
  (params (OverlappedComponent :type "PrimitiveComponent Object Reference") (OtherActor :type "Actor Object Reference") (OtherComp :type "PrimitiveComponent Object Reference") (OtherBodyIndex :type Integer) (bFromSweep :type Boolean) (SweepResult :type "HitResult Structure (by ref)"))
  (cast `/Game/ThirdPersonBP/Blueprints/ThirdPersonCharacterAlternative` OtherActor)
  (bind _aspeace_game (cast `/Game/Assets/Blueprints/GameInstance/PeaceGame` (`GameplayStatics.GetGameInstance`)))
  (if (>= (`/Game/Assets/Blueprints/GameInstance/PeaceGame.AllMemoriesMended` _aspeace_game) 3)
    (bind (_direction _fade) (`Timeline|Timeline_0`)
      (:`Update`
        (`SceneComponent.SetRelativeScale3D` (`self.ParticleSystem`) (`KismetMathLibrary.Conv_DoubleToVector` _fade))
        (`KismetSystemLibrary.Delay` 1.0)
        (`SceneComponent.SetVisibility` null true false)
        (`SceneComponent.SetVisibility` (`self.ParticleSystem`) true false)
        (`SceneComponent.SetVisibility` (`self.Plane`) true false)
        (`KismetSystemLibrary.Delay` 2.5)
        (bind (_outactor _returnvalue) (`LevelSequencePlayer.CreateLevelSequencePlayer` "/Game/EndCutscene.EndCutscene"))))
    (else
      (`SceneComponent.SetVisibility` (`self.Pictogram`) true false))))

(event `self.Box.OnComponentEndOverlap`
  (params (OverlappedComponent :type "PrimitiveComponent Object Reference") (OtherActor :type "Actor Object Reference") (OtherComp :type "PrimitiveComponent Object Reference") (OtherBodyIndex :type Integer))
  (cast `/Game/ThirdPersonBP/Blueprints/ThirdPersonCharacterAlternative` OtherActor)
  (`KismetSystemLibrary.Delay` 2.0)
  (`SceneComponent.SetVisibility` null false false)
  (`SceneComponent.SetVisibility` (`self.Pictogram`) false false)
  (`SceneComponent.SetVisibility` (`self.Plane`) false false))

(fn `UserConstructionScript`)