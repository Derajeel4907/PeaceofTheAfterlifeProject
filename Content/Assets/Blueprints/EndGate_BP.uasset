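; End gate actor that reacts to the player entering its trigger box based on the PeaceGame instance's MemoryPickup flag.
; With the memory, it shows a text bubble and scales its particle system through a timeline before destroying it; otherwise it shows a pictogram bubble.
; A self-recalling 0.01-second delay loop yaws the text toward the player, and leaving the box hides the bubble after a delay.
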(event `Speech Bubble Rotation`
  (bind _textrender (`self.TextRender`))
  (bind (_returnvalue_roll _returnvalue_pitch _returnvalue_yaw) (`KismetMathLibrary.BreakRotator` (`KismetMathLibrary.FindLookAtRotation` (`SceneComponent.K2_GetComponentLocation` _textrender) (`self.K2_GetActorLocation` (stale `self.Box.OnComponentBeginOverlap` _asthird_person_character_alternative)))))
  (`SceneComponent.K2_SetRelativeRotation` _textrender (`KismetMathLibrary.MakeRotator` 0.0 0.0 _returnvalue_yaw) false false)
  (`KismetSystemLibrary.Delay` 0.01)
  (`self.Speech Bubble Rotation`))

(event `self.Box.OnComponentBeginOverlap`
  (params (OverlappedComponent :type "PrimitiveComponent Object Reference") (OtherActor :type "Actor Object Reference") (OtherComp :type "PrimitiveComponent Object Reference") (OtherBodyIndex :type Integer) (bFromSweep :type Boolean) (SweepResult :type "HitResult Structure (by ref)"))
  (bind _particlesystem (`self.ParticleSystem`))
  (bind _asthird_person_character_alternative (cast `/Game/ThirdPersonBP/Blueprints/ThirdPersonCharacterAlternative` OtherActor))
  (`self.Speech Bubble Rotation`)
  (bind _aspeace_game (cast `/Game/Assets/Blueprints/GameInstance/PeaceGame` (`GameplayStatics.GetGameInstance`)))
  (if (`/Game/Assets/Blueprints/GameInstance/PeaceGame.MemoryPickup` _aspeace_game)
    (`SceneComponent.SetVisibility` (`self.TextRender`) true false)
    (`SceneComponent.SetVisibility` (`self.Cube`) true false)
    (bind (_direction _fade) (`Timeline|Timeline_0`)
      (:`Update`
        (`SceneComponent.SetRelativeScale3D` _particlesystem (`KismetMathLibrary.Conv_DoubleToVector` _fade))
        (`KismetSystemLibrary.Delay` 1.0)
        (`ActorComponent.K2_DestroyComponent` _particlesystem)))
    (else
      (`SceneComponent.SetVisibility` (`self.Cube`) true false)
      (`SceneComponent.SetVisibility` (`self.Pictogram`) true false))))

(event `self.Box.OnComponentEndOverlap`
  (params (OverlappedComponent :type "PrimitiveComponent Object Reference") (OtherActor :type "Actor Object Reference") (OtherComp :type "PrimitiveComponent Object Reference") (OtherBodyIndex :type Integer))
  (cast `/Game/ThirdPersonBP/Blueprints/ThirdPersonCharacterAlternative` OtherActor)
  (`KismetSystemLibrary.Delay` 2.0)
  (`SceneComponent.SetVisibility` (`self.Cube`) false false)
  (`SceneComponent.SetVisibility` (`self.TextRender`) false false)
  (`SceneComponent.SetVisibility` (`self.Pictogram`) false false))

(fn `UserConstructionScript`)